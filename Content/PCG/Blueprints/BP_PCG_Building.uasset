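; BP_PCG_Building is an actor that configures a PCG graph, apparently for generating a multi-layer building.
; Its Construction Script turns Spacing into half-spacing wall offsets, along Y for forward and backward and along X for left and right.
; It writes these offsets, plus LayerNum and LayerHeight, into the PCG component's graph instance parameters.
; The event graph holds only disabled placeholder events, so the Blueprint adds no runtime logic.
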(event EventBeginPlay)

(event Collision|EventActorBeginOverlap
  (params (OtherActor :type Actor%20Object%20Reference)))

(event EventTick
  (params (DeltaSeconds :type Float%20%28single-precision%29)))

(fn ConstructionScript
  (bind _pcg (Variables|Default|GetPCG))
  (bind _spacing (Variables|Default|GetSpacing))
  (bind _returnvalue (/ _spacing -2.0))
  (bind _returnvalue_2 (/ _spacing 2.0))
  (bind _graphinstance (Variables|/Script/PCG.PCGComponent|GetGraphInstance _pcg))
  (Effects|Components|ParticleSystem|SetVectorParameter _graphinstance "WallOffestFwd" (Math|Vector|MakeVector 0.0 _returnvalue_2 0.0))
  (Effects|Components|ParticleSystem|SetVectorParameter _graphinstance "WallOffestBwd" (Math|Vector|MakeVector 0.0 _returnvalue 0.0))
  (Effects|Components|ParticleSystem|SetVectorParameter _graphinstance "WallOffestLeft" (Math|Vector|MakeVector _returnvalue 0.0 0.0))
  (Effects|Components|ParticleSystem|SetVectorParameter _graphinstance "WallOffestRight" (Math|Vector|MakeVector _returnvalue_2 0.0 0.0))
  (Class|PCGGraphParametersHelpers|SetInt32Parameter _graphinstance "LayerNum" (Variables|Default|GetLayerNum))
  (Effects|Components|ParticleSystem|SetFloatParameter _graphinstance "LayerHeight" (Variables|Default|GetLayerHeight)))